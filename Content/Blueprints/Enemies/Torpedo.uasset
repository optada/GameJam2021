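; Enemy torpedo that propels itself by applying forward force to its mesh each tick while its Target is valid, with no steering in this graph.
; Hits on Ships are ignored here; any other hit detonates the torpedo, first triggering Explosion on the other actor if it is a DamageInstigator.
; The Explosion override plays a water sound at the torpedo's location before calling the parent implementation.
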(event `self.ReceiveTick`
  (params (DeltaSeconds :type "Float (single-precision)"))
  (bind _torpedomesh (`self.TorpedoMesh`))
  (`/Engine/EditorBlueprintResources/StandardMacros.IsValid` (`self.Target`)
    (:`Is Valid`
      (`PrimitiveComponent.AddForce` _torpedomesh (* (`SceneComponent.GetForwardVector` _torpedomesh) (`self.MoveForce`)) "None" false))))

(event `self.TorpedoMesh.OnComponentHit`
  (params (HitComponent :type "PrimitiveComponent Object Reference") (OtherActor :type "Actor Object Reference") (OtherComp :type "PrimitiveComponent Object Reference") (NormalImpulse :type "Vector Structure") (Hit :type "HitResult Structure (by ref)"))
  (cast `/Game/Blueprints/Player/Ships` OtherActor
    (:`CastFailed`
      (bind _asdamage_instigator (cast `/Game/Blueprints/Enemies/DamageInstigator` OtherActor)
        (:`then`
          (`self.Explosion` _asdamage_instigator))
        (:`CastFailed`
          _))
      (`self.Explosion`))))

(fn `Explosion`
  (`GameplayStatics.PlaySoundAtLocation` "/Game/Sound/Water_aftershoot_Cue.Water_aftershoot_Cue" (`self.K2_GetActorLocation`) (struct) 1.0 1.0 0.0 null null null)
  (`parent.Explosion`))

(fn `UserConstructionScript`)