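; Player controller that relays movement input for two sets of controls to a single Ships reference.
; Forward and turn axes for each set pass straight to matching functions on Ships, which holds the movement logic.
; SetupCamera makes Ships the view target when it is valid, though nothing in this graph calls it.
; Escape or J opens level LVL_00.
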(event `Key|Escape`
  (params (Key :type "Key Structure"))
  (:`Pressed`
    (`GameplayStatics.OpenLevel` "LVL_00" :!label _label)))

(event `Key|J`
  (params (Key :type "Key Structure"))
  (:`Pressed`
    (goto _label)))

(event `InputAxis|MoveForward1`
  (params (AxisValue :type "Float (single-precision)"))
  (`/Game/Blueprints/Player/Ships.MoveForward1Ship` (`self.Ships`) AxisValue))

(event `InputAxis|MoveForward2`
  (params (AxisValue :type "Float (single-precision)"))
  (`/Game/Blueprints/Player/Ships.MoveForward2Ship` (`self.Ships`) AxisValue))

(event `InputAxis|TurnRight1`
  (params (AxisValue :type "Float (single-precision)"))
  (`/Game/Blueprints/Player/Ships.TurnRight1Ship` (`self.Ships`) AxisValue))

(event `InputAxis|TurnRight2`
  (params (AxisValue :type "Float (single-precision)"))
  (`/Game/Blueprints/Player/Ships.TurnRight2Ship` (`self.Ships`) AxisValue))

(fn `SetupCamera`
  (bind _ships (`self.Ships`))
  (`/Engine/EditorBlueprintResources/StandardMacros.IsValid` _ships
    (:`Is Valid`
      (`self.SetViewTargetWithBlend` _ships))))

(fn `UserConstructionScript`)