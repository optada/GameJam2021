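; Player actor holding two physics-driven ships, their health and a shared camera that follows their horizontal midpoint at constant height.
; Movement functions push each ship along its forward vector and apply yaw torque scaled by current speed, so turning needs momentum.
; Hits from DamageInstigator actors subtract health and trigger their explosion.
; Tick updates both health widgets and restarts the ShipsGameMode once either ship runs out of health.
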(event `self.ReceiveTick`
  (params (DeltaSeconds :type "Float (single-precision)"))
  (bind _playercamera (`self.PlayerCamera`))
  (bind (_returnvalue_x _returnvalue_y _returnvalue_z) (`KismetMathLibrary.BreakVector` (`SceneComponent.K2_GetComponentLocation` _playercamera)))
  (bind (_returnvalue_x_2 _returnvalue_y_2) (`KismetMathLibrary.BreakVector` (/ (+ (`SceneComponent.K2_GetComponentLocation` (`self.Ship1`)) (`SceneComponent.K2_GetComponentLocation` (`self.Ship2`))) 2.0)))
  (`SceneComponent.K2_SetWorldLocation` _playercamera (`KismetMathLibrary.MakeVector` _returnvalue_x_2 _returnvalue_y_2 _returnvalue_z) false false)
  (if (and (> (`self.ShipHealth1`) 0.0) (> (`self.ShipHealth2`) 0.0))
    (bind _ashealth_widget (cast `/Game/Blueprints/Player/HealthWidget` (`WidgetComponent.GetWidget` (`self.Health1`))))
    (`/Game/Blueprints/Player/HealthWidget.Init` _ashealth_widget false)
    (`ProgressBar.SetPercent` (`/Game/Blueprints/Player/HealthWidget.ProgressBar_0` _ashealth_widget) (/ (`self.ShipHealth1`) 100.0))
    (bind _ashealth_widget_2 (cast `/Game/Blueprints/Player/HealthWidget` (`WidgetComponent.GetWidget` (`self.Health2`))))
    (`/Game/Blueprints/Player/HealthWidget.Init` _ashealth_widget_2 true)
    (`ProgressBar.SetPercent` (`/Game/Blueprints/Player/HealthWidget.ProgressBar_0` _ashealth_widget_2) (/ (`self.ShipHealth2`) 100.0))
    (else
      (bind _asships_game_mode (cast `/Game/Blueprints/ShipsGameMode` (`GameplayStatics.GetGameMode`)))
      (`/Game/Blueprints/ShipsGameMode.Restart` _asships_game_mode))))

(event `self.Ship1.OnComponentHit`
  (params (HitComponent :type "PrimitiveComponent Object Reference") (OtherActor :type "Actor Object Reference") (OtherComp :type "PrimitiveComponent Object Reference") (NormalImpulse :type "Vector Structure") (Hit :type "HitResult Structure (by ref)"))
  (bind _asdamage_instigator (cast `/Game/Blueprints/Enemies/DamageInstigator` OtherActor))
  (bind _output_get (set `self.ShipHealth1` (- (`self.ShipHealth1`) (`/Game/Blueprints/Enemies/DamageInstigator.Damage` _asdamage_instigator))))
  (`/Game/Blueprints/Enemies/DamageInstigator.Explosion` _asdamage_instigator)
  (`KismetSystemLibrary.PrintString` (`KismetStringLibrary.Conv_DoubleToString` _output_get) true true (struct :`R` 1.0 :`G` 0.08042 :`A` 1.0)))

(event `self.Ship2.OnComponentHit`
  (params (HitComponent :type "PrimitiveComponent Object Reference") (OtherActor :type "Actor Object Reference") (OtherComp :type "PrimitiveComponent Object Reference") (NormalImpulse :type "Vector Structure") (Hit :type "HitResult Structure (by ref)"))
  (bind _asdamage_instigator (cast `/Game/Blueprints/Enemies/DamageInstigator` OtherActor))
  (bind _output_get (set `self.ShipHealth2` (- (`self.ShipHealth2`) (`/Game/Blueprints/Enemies/DamageInstigator.Damage` _asdamage_instigator))))
  (`/Game/Blueprints/Enemies/DamageInstigator.Explosion` _asdamage_instigator)
  (`KismetSystemLibrary.PrintString` (`KismetStringLibrary.Conv_DoubleToString` _output_get) true true (struct :`R` 1.0 :`G` 0.08042 :`A` 1.0)))

(fn `ApplyForceToShip`
  (params (Ship :type "PrimitiveComponent Object Reference") (Input :type "Float (double-precision)") (ShipPower :type "Float (double-precision)"))
  (`PrimitiveComponent.AddForce` Ship (* (`SceneComponent.GetForwardVector` Ship) (* Input ShipPower)) "None" false))

(fn `ApplyRotateForceToShip`
  (params (Ship :type "PrimitiveComponent Object Reference") (RightSideInput :type "Float (double-precision)") (RotatePower :type "Float (double-precision)"))
  (bind _returnvalue (`PrimitiveComponent.GetPhysicsLinearVelocity` Ship "None"))
  (`PrimitiveComponent.AddTorqueInDegrees` Ship (`KismetMathLibrary.MakeVector` 0.0 0.0 (* (/ (`KismetMathLibrary.VSize` _returnvalue) 4.0) (* RightSideInput RotatePower))) "None" false))

(fn `MoveForward1Ship`
  (params (Input :type "Float (double-precision)"))
  (`self.ApplyForceToShip` (`self.Ship1`) Input (`self.MainEngineForce`)))

(fn `MoveForward2Ship`
  (params (Input :type "Float (double-precision)"))
  (`self.ApplyForceToShip` (`self.Ship2`) Input (`self.MainEngineForce`)))

(fn `TurnRight1Ship`
  (params (Input :type "Float (double-precision)"))
  (`self.ApplyRotateForceToShip` (`self.Ship1`) Input (`self.MainRotateForce`)))

(fn `TurnRight2Ship`
  (params (Input :type "Float (double-precision)"))
  (`self.ApplyRotateForceToShip` (`self.Ship2`) Input (`self.MainRotateForce`)))

(fn `UserConstructionScript`)