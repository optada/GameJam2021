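; Game mode for a ship game that spawns the player's two-ship actor, links it to the main controller's camera, and spawns watermine and torpedo hazards.
; While playing, Tick raises a difficulty counter that increases the random chance of spawning hazards around the camera within distance bands.
; Each torpedo spawns facing a randomly chosen ship, which becomes its target.
; Restart resets the level, respawns the ships and destroys DamageInstigator actors.
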(event `self.ReceiveBeginPlay`
  (bind _mainships (`self.MainShips`))
  (bind _asmain_player_controller (cast `/Game/Blueprints/Player/MainPlayerController` (`GameplayStatics.GetPlayerController` 0)))
  (set `self.MainController` _asmain_player_controller)
  (`self.SpawnMainShips`)
  (`self.SpawnWatermine` 500.0 500.0 :!label _label)
  (`self.SpawnTorpedo` -1000.0 -800.0 (select `bool` (`KismetMathLibrary.RandomBool`) :`false` (`/Game/Blueprints/Player/Ships.Ship1` _mainships) :`true` (`/Game/Blueprints/Player/Ships.Ship2` _mainships))))

(event `OnRestart`
  (goto _label))

(event `self.ReceiveTick`
  (params (DeltaSeconds :type "Float (single-precision)"))
  (if (`self.IsPlaing`)
    (bind _output_get (set `self.TTDK` (+ (`self.TTDK`) 0.0005)))
    (`self.GenerateMines` (+ _output_get (`self.MineRandom`)) 2500.0 2000.0)
    (`self.GenerateTorpedos` (+ _output_get (`self.TorpedRandom`)) 2000.0 1500.0)))

(fn `GenerateMines`
  (params (Random :type "Float (double-precision)") (MaxDistance :type "Float (double-precision)") (MinDistance :type "Float (double-precision)"))
  (bind (_succesfull _x _y) (`self.GenerateCoordinatesForObject` MaxDistance MinDistance))
  (if (and (`KismetMathLibrary.RandomBoolWithWeight` Random) _succesfull)
    (`self.SpawnWatermine` _x _y)))

(fn `GenerateTorpedos`
  (params (Random :type "Float (double-precision)") (MaxDistance :type "Float (double-precision)") (MinDistance :type "Float (double-precision)"))
  (bind (_succesfull _x _y) (`self.GenerateCoordinatesForObject` MaxDistance MinDistance))
  (bind _mainships (`self.MainShips`))
  (if (and (`KismetMathLibrary.RandomBoolWithWeight` Random) _succesfull)
    (`self.SpawnTorpedo` _x _y (select `bool` (`KismetMathLibrary.RandomBool`) :`false` (`/Game/Blueprints/Player/Ships.Ship1` _mainships) :`true` (`/Game/Blueprints/Player/Ships.Ship2` _mainships)))))

(fn `OnLoose`)

(fn `Restart`
  (bind _mainships (`self.MainShips`))
  (`self.ResetLevel`)
  (`/Engine/EditorBlueprintResources/StandardMacros.IsValid` _mainships
    (:`Is Valid`
      (`self.K2_DestroyActor` _mainships))
    (:`Is Not Valid`
      _))
  (`self.SpawnMainShips`)
  (`self.OnRestart`)
  (bind _outactors (`GameplayStatics.GetAllActorsOfClass` "/Game/Blueprints/Enemies/DamageInstigator.DamageInstigator_C"))
  (for _array_element _outactors
    (`self.K2_DestroyActor` _array_element)))

(fn `SpawnMainShips`
  (bind _maincontroller (`self.MainController`))
  (bind _returnvalue (`|SpawnActorFromClass` "/Game/Blueprints/Player/Ships.Ships_C" (`KismetMathLibrary.MakeTransform` (`KismetMathLibrary.MakeVector` 0.0 0.0 (`self.Z_Level`))) "AlwaysSpawn" "OverrideRootScale" _maincontroller null))
  (bind _output_get (set `/Game/Blueprints/Player/MainPlayerController.Ships` _returnvalue _maincontroller))
  (bind _output_get_2 (set `self.MainShips` _output_get))
  (`/Game/Blueprints/Player/MainPlayerController.SetupCamera` _maincontroller)
  (`/Engine/EditorBlueprintResources/StandardMacros.IsValid` _output_get_2
    (:`Is Valid`
      (`KismetSystemLibrary.PrintString` "ShipSpawned" true true (struct :`R` 0.052967 :`G` 1.0 :`A` 1.0) 3.0))
    (:`Is Not Valid`
      (`KismetSystemLibrary.PrintString` "Can not create ships" true true (struct :`R` 1.0 :`A` 1.0) 10.0))))

(fn `SpawnTorpedo`
  (params (X :type "Float (double-precision)") (Y :type "Float (double-precision)") (Target :type "PrimitiveComponent Object Reference"))
  (bind _returnvalue (- (`self.Z_Level`) 10.0))
  (bind _returnvalue_2 (`|SpawnActorFromClass` "/Game/Blueprints/Enemies/Torpedo.Torpedo_C" (`KismetMathLibrary.MakeTransform` (`KismetMathLibrary.MakeVector` X Y _returnvalue) (`KismetMathLibrary.FindLookAtRotation` (`KismetMathLibrary.MakeVector` X Y _returnvalue) (`SceneComponent.K2_GetComponentLocation` Target))) "Undefined" "OverrideRootScale" null null))
  (`/Engine/EditorBlueprintResources/StandardMacros.IsValid` _returnvalue_2
    (:`Is Valid`
      (set `/Game/Blueprints/Enemies/DamageInstigator.Target` Target _returnvalue_2))))

(fn `SpawnWatermine`
  (params (X :type "Float (double-precision)") (Y :type "Float (double-precision)"))
  (`|SpawnActorFromClass` "/Game/Blueprints/Enemies/Watermine.Watermine_C" (`KismetMathLibrary.MakeTransform` (`KismetMathLibrary.MakeVector` X Y (- (`self.Z_Level`) 5.0))) "Undefined" "OverrideRootScale" null null))

(fn `UserConstructionScript`)